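; Ghost character that collects all patrol point actors at BeginPlay and can be reset to its starting transform, with no patrol logic in this Blueprint.
; Construction tints the mesh through a dynamic material, saves the transform and derives walk speed from the GameInstance level via a math expression.
; Reset teleports it back and restores NavWalking, while SetMovementEnabled always disables movement, ignoring its Enabled input.
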(event EventBeginPlay
  (bind _outactors (Actor|GetAllActorsOfClass "/Game/Blueprints/BP_PatrolPoint.BP_PatrolPoint_C"))
  (Variables|Default|SetPatrolPoints _outactors))

(fn ConstructionScript
  (bind _returnvalue (Rendering|Material|CreateDynamicMaterialInstance (Variables|Character|GetMesh) 0 0 "None" :!class /Script/Engine.PrimitiveComponent))
  (Rendering|Material|SetVectorParameterValue _returnvalue "BaseColor" (Math|Conversions|ToLinearColor(Color) (Variables|Default|GetColor)) :!class /Script/Engine.MaterialInstanceDynamic)
  (CallFunction|UpdateWalkSpeed)
  (Variables|Default|SetOriginalTransform (Transformation|GetActorTransform)))

(fn UpdateWalkSpeed
  (bind _asbp_game_instance (Utilities|Casting|CastToBP_GameInstance (Game|GetGameInstance)))
  (Variables|/Script/Engine.CharacterMovementComponent|SetMaxWalkSpeed (Variables|Character|GetCharacterMovement) (|(((Level-1)*{EC79BA18-D245-18C9-E120-598A8B228EC3})+{834F6B65-F747-0A5A-E266-8787B6ACFF00}) (Math|Conversions|ToFloat(Integer) (Variables|/Game/Blueprints/BP_GameInstance.BP_GameInstance_C|GetLevel _asbp_game_instance)))))

(fn Reset
  (Transformation|SetActorTransform (Variables|Default|GetOriginalTransform) false true)
  (Pawn|Components|CharacterMovement|SetMovementMode (Variables|Character|GetCharacterMovement) "MOVE_NavWalking" 0))

(fn SetMovementEnabled
  (params (Enabled :type Boolean))
  (Pawn|Components|CharacterMovement|DisableMovement (Variables|Character|GetCharacterMovement)))