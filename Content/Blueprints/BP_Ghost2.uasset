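; BP_Ghost2 is a ghost that tracks patrol points and tints its mesh with a configurable color.
; On BeginPlay it fills PatrolPoints with every BP_PatrolPoint in the level.
; Overlaps on PatrolPointsCollision then add or remove points from that array, printing debug strings, though no patrol movement happens in these graphs.
; The construction script applies Color to the BaseColor parameter of a dynamic material instance.
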(event OnComponentBeginOverlap(PatrolPointsCollision)
  (params (OverlappedComponent :type Primitive%20Component%20Object%20Reference) (OtherActor :type Actor%20Object%20Reference) (OtherComp :type Primitive%20Component%20Object%20Reference) (OtherBodyIndex :type Integer) (bFromSweep :type Boolean) (SweepResult :type Hit%20Result%20Structure%20%28by%20ref%29))
  (bind _asbp_patrol_point (Utilities|Casting|CastToBP_PatrolPoint OtherActor))
  (Development|PrintString "Test")
  (Utilities|Array|AddUnique (Variables|Default|GetPatrolPoints) _asbp_patrol_point)
  (Development|PrintString "Adding patrol point"))

(event OnComponentEndOverlap(PatrolPointsCollision)
  (params (OverlappedComponent :type Primitive%20Component%20Object%20Reference) (OtherActor :type Actor%20Object%20Reference) (OtherComp :type Primitive%20Component%20Object%20Reference) (OtherBodyIndex :type Integer))
  (bind _asbp_patrol_point (Utilities|Casting|CastToBP_PatrolPoint OtherActor))
  (Utilities|Array|RemoveItem (Variables|Default|GetPatrolPoints) _asbp_patrol_point)
  (Development|PrintString "Removing patrol point"))

(event EventBeginPlay
  (bind _outactors (Actor|GetAllActorsOfClass "/Game/Blueprints/BP_PatrolPoint.BP_PatrolPoint_C"))
  (Variables|Default|SetPatrolPoints _outactors))

(event Collision|EventActorBeginOverlap
  (params (OtherActor :type Actor%20Object%20Reference)))

(event EventTick
  (params (DeltaSeconds :type Float%20%28single-precision%29)))

(fn ConstructionScript
  (bind _returnvalue (Rendering|Material|CreateDynamicMaterialInstance (Variables|Character|GetMesh) 0 0 "None" :!class /Script/Engine.PrimitiveComponent))
  (Rendering|Material|SetVectorParameterValue _returnvalue "BaseColor" (Math|Conversions|ToLinearColor(Color) (Variables|Default|GetColor)) :!class /Script/Engine.MaterialInstanceDynamic))