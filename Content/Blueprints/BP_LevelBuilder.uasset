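; Level builder Blueprint for a Paper2D tile map named TMPacman, apparently meant to build a Pac-Man level, though the building is not yet implemented.
; BeginPlay caches the tile map's width and height.
; BuildLevelFromTileMap and the construction script are empty.
; Disconnected nodes probe a single tile's index and user data, the latter feeding an empty switch.
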(event EventBeginPlay
  (bind _tm_pacman (Variables|Default|GetTM_Pacman))
  (bind _tilemap (Variables|/Script/Paper2D.PaperTileMapComponent|GetTileMap _tm_pacman))
  (Variables|Default|SetTileMapWidth (Variables|/Script/Paper2D.PaperTileMap|GetMapWidth _tilemap))
  (Variables|Default|SetTileMapHeight (Variables|/Script/Paper2D.PaperTileMap|GetMapHeight _tilemap)))

(fn ConstructionScript)

(fn BuildLevelfromTileMap)