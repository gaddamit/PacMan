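; Tile map level Blueprint, apparently an early stub for constructing a level from a Paper2D tile map.
; The construction script assigns the tile map to the render component, and BeginPlay caches its width and height.
; ContructLevelFromTileMap only prints each layer 0 tile index, passing the height counter as X and width as Y, then prints a debug string.
; Nothing here calls that function or spawns geometry.
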(event EventBeginPlay
  (bind _rendercomponent (Variables|Default|GetRenderComponent))
  (bind _tilemap (Variables|/Script/Paper2D.PaperTileMapComponent|GetTileMap _rendercomponent))
  (Variables|Default|SetMapWidth (Variables|/Script/Paper2D.PaperTileMap|GetMapWidth _tilemap))
  (Variables|Default|SetMapHeight (Variables|/Script/Paper2D.PaperTileMap|GetMapHeight _tilemap)))

(fn ConstructionScript
  (Class|PaperTileMapComponent|SetTileMap (Variables|Default|GetRenderComponent) (Variables|Default|GetPaper%20Tile%20Map)))

(fn ContructLevelfromTileMap
  (for _index (range 0 (- (Variables|Default|GetMapHeight) 1))
    (for _index_2 (range 0 (- (Variables|Default|GetMapWidth) 1))
      (Development|PrintString (Utilities|String|ToString(Integer) (.tileindex (Class|PaperTileMapComponent|GetTile (Variables|Default|GetRenderComponent) _index _index_2))))))
  (Development|PrintString "Hello"))