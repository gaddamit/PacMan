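; BP_Pacman is the Pac-Man actor, whose only logic here is teleporting between portals.
; Teleport runs once while HasTeleported is false, sets that flag, disables overlap events on the previous portal and moves the capsule to the destination portal's root location.
; Nothing in this graph calls Teleport or resets the flag, and the default event nodes are disabled.
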(event EventBeginPlay
  (|CallParentFunction) ; This node is disabled and will not be called.\nDrag off pins to build functionality.
)

(event Collision|EventActorBeginOverlap
  (params (OtherActor :type Actor%20Object%20Reference)))

(event EventTick
  (params (DeltaSeconds :type Float%20%28single-precision%29)))

(fn ConstructionScript
  (|CallParentFunction))

(fn Teleport
  (params (PreviousPortal :type BP%20Portal%20Object%20Reference) (Portal :type BP%20Portal%20Object%20Reference))
  (if (not (Variables|Default|GetHasTeleported))
    (Variables|Default|SetHasTeleported true)
    (Default|SetOverlapEvents PreviousPortal false)
    (Transformation|SetWorldLocationAndRotation (Variables|Default|GetCapsuleComponent) (Transformation|GetWorldLocation (Variables|/Game/Blueprints/BP_Portal.BP_Portal_C|GetDefaultSceneRoot Portal)) "0, 0, 0" false true)))