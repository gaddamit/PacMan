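; BP_Pellet2 is a pellet actor with a glowing sphere mesh in a configurable color.
; Its construction script creates a dynamic material instance of M_Glowing on the Sphere and sets its BaseColor parameter from the Color variable.
; The event graph holds only disabled default events, so the Blueprint adds no gameplay logic there.
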(event EventBeginPlay
  (|CallParentFunction) ; This node is disabled and will not be called.\nDrag off pins to build functionality.
)

(event Collision|EventActorBeginOverlap
  (params (OtherActor :type Actor%20Object%20Reference))
  (|CallParentFunction OtherActor) ; This node is disabled and will not be called.\nDrag off pins to build functionality.
)

(event EventTick
  (params (DeltaSeconds :type Float%20%28single-precision%29))
  (|CallParentFunction DeltaSeconds) ; This node is disabled and will not be called.\nDrag off pins to build functionality.
)

(fn ConstructionScript
  (|CallParentFunction)
  (bind _returnvalue (Rendering|Material|CreateDynamicMaterialInstance (Variables|Default|GetSphere) 0 "/Game/Materials/M_Glowing.M_Glowing" "None" :!class /Script/Engine.PrimitiveComponent))
  (Rendering|Material|SetVectorParameterValue _returnvalue "BaseColor" (Math|Conversions|ToLinearColor(Color) (Variables|Default|GetColor)) :!class /Script/Engine.MaterialInstanceDynamic))