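; BP_TileMap is a Paper2D tile map actor that scans its map at construction, apparently as groundwork for building a level from tiles.
; The construction script caches the render component's tile map and dimensions, then calls ContructLevelFromTileMap.
; That function only prints each layer 0 tile index so far, passing the height counter as X and the width counter as Y.
; BeginPlay just prints a debug string.
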(event EventBeginPlay
  (Development|PrintString "Hello2"))

(event Collision|EventActorBeginOverlap
  (params (OtherActor :type Actor%20Object%20Reference)))

(event EventTick
  (params (DeltaSeconds :type Float%20%28single-precision%29)))

(fn ConstructionScript
  (Development|PrintString "Hello")
  (bind _output_get (Variables|Default|SetPaper%20Tile%20Map (Variables|/Script/Paper2D.PaperTileMapComponent|GetTileMap (Variables|Default|GetRenderComponent))))
  (Variables|Default|SetMapWidth (Variables|/Script/Paper2D.PaperTileMap|GetMapWidth _output_get))
  (Variables|Default|SetMapHeight (Variables|/Script/Paper2D.PaperTileMap|GetMapHeight _output_get))
  (Development|PrintString (Utilities|String|ToString(Integer) (Variables|/Script/Paper2D.PaperTileMap|GetMapWidth _output_get)))
  (CallFunction|ContructLevelfromTileMap))

(fn ContructLevelfromTileMap
  (for _index (range 0 (- (Variables|Default|GetMapHeight) 1))
    (for _index_2 (range 0 (- (Variables|Default|GetMapWidth) 1))
      (Development|PrintString (Utilities|String|ToString(Integer) (.tileindex (Class|PaperTileMapComponent|GetTile (Variables|Default|GetRenderComponent) _index _index_2))))))
  (Development|PrintString "Hello"))